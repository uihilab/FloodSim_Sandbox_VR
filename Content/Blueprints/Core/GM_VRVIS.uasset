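; Game mode for a flood simulation that picks the player's pawn based on the ViewInVR flag stored on the Floodsim game instance.
; SpawnDefaultPawnFor spawns either BP_VRPlayer or BP_FPSPlayer at the world origin, ignoring the start spot, and prints a message if the cast fails.
; SubmitConfig makes a similar choice using VRPawn and possesses the result, but its only call in the event graph is disconnected.
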(event `self.ReceiveBeginPlay`)

(fn `SpawnDefaultPawnFor`
  (params (NewPlayer :type "Controller Object Reference") (StartSpot :type "Actor Object Reference"))
  (returns (ReturnValue :type "Pawn Object Reference"))
  (bind _returnvalue (`KismetMathLibrary.MakeTransform` (0.0 0.0 0.0)))
  (bind _asfloodsim (cast `Floodsim` (`GameplayStatics.GetGameInstance`))
    (:`then`
      (if (`Floodsim.ViewInVR` _asfloodsim)
        (bind _returnvalue_2 (`|SpawnActorFromClass` "/Game/Blueprints/Player/BP_VRPlayer.BP_VRPlayer_C" _returnvalue "Undefined" "MultiplyWithRoot" null null))
        (set `self.PlayerChar` _returnvalue_2)
        (else
          (bind _returnvalue_3 (`|SpawnActorFromClass` "/Game/Blueprints/Player/BP_FPSPlayer.BP_FPSPlayer_C" _returnvalue "Undefined" "MultiplyWithRoot" null null))
          (set `self.PlayerChar` _returnvalue_3)))
      (return (`self.PlayerChar`)))
    (:`CastFailed`
      (`KismetSystemLibrary.PrintString` "Cast failed."))))

(fn `SubmitConfig`
  (bind _returnvalue (`KismetMathLibrary.MakeTransform` (0.0 0.0 0.0)))
  (bind _returnvalue_2 (`GameplayStatics.GetPlayerController` 0))
  (bind _asfloodsim (cast `Floodsim` (`GameplayStatics.GetGameInstance`)))
  (if (`Floodsim.ViewInVR` _asfloodsim)
    (bind _returnvalue_3 (`|SpawnActorFromClass` "/Game/VRTemplate/Blueprints/VRPawn.VRPawn_C" _returnvalue "Undefined" "MultiplyWithRoot" null null))
    (`Controller.Possess` _returnvalue_2 _returnvalue_3)
    (else
      (bind _returnvalue_4 (`|SpawnActorFromClass` "/Game/Blueprints/Player/BP_FPSPlayer.BP_FPSPlayer_C" _returnvalue "Undefined" "MultiplyWithRoot" null null))
      (`Controller.Possess` _returnvalue_2 _returnvalue_4))))

(fn `UserConstructionScript`)