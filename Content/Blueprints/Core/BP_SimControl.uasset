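; BP_SimControl is the central controller for a flood simulation scene with an FPS or VR player.
; On BeginPlay it caches scene actors, then recomputes content and structure damage every half second from fluid height using clamped linear functions.
; It exposes play/pause, reset, timelapse via raised iteration rates, building inundation toggling and player teleporting.
; Other functions drive SkyCreator weather and time, Flux source discharge and floodmap height.
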(event `ChangeSim`
  (`/Game/FluidFlux/Simulation/Blueprints/BP_FluxSimulationDomain.ToggleUpdateSimulation` (`self.SimDomain`)))

(event `self.ReceiveBeginPlay`
  (bind _outactors (`GameplayStatics.GetAllActorsWithTag` "Building"))
  (set `self.Buildings` _outactors)
  (bind _returnvalue (`GameplayStatics.GetActorOfClass` "/Game/FluidFlux/Simulation/Blueprints/BP_FluxSimulationDomain.BP_FluxSimulationDomain_C"))
  (set `self.SimDomain` _returnvalue)
  (bind _returnvalue_2 (`GameplayStatics.GetActorOfClass` "/Script/SkyCreatorPlugin.SkyCreator"))
  (set `self.SkyRef` _returnvalue_2)
  (bind _returnvalue_3 (`GameplayStatics.GetActorOfClass` "/Game/FluidFlux/Simulation/Modifiers/BP_FluxModifierSourceActor.BP_FluxModifierSourceActor_C"))
  (set `self.SceneMod` _returnvalue_3)
  (bind _returnvalue_4 (`GameplayStatics.GetActorOfClass` "/Game/Blueprints/Player/BP_FPSPlayer.BP_FPSPlayer_C"))
  (`/Engine/EditorBlueprintResources/StandardMacros.IsValid` _returnvalue_4
    (:`Is Valid`
      (set `self.PlayerChar` _returnvalue_4)
      (bind _outactors_2 (`GameplayStatics.GetAllActorsOfClass` "/Game/VehicleTemplate/Blueprints/SportsCar/AI_Car.AI_Car_C" :!label _label))
      (set `self.Vehicles` _outactors_2)
      (bind _outactors_3 (`GameplayStatics.GetAllActorsOfClass` "/Game/Blueprints/NPCs/Humans/AI_Human.AI_Human_C"))
      (set `self.Humans` _outactors_3)
      (bind _returnvalue_5 (`GameplayStatics.GetActorOfClass` "/Game/Blueprints/BP_Floodmap.BP_Floodmap_C"))
      (bind _output_get (set `self.Floodmap` _returnvalue_5))
      (bind (_returnvalue_x _returnvalue_y _returnvalue_z) (`KismetMathLibrary.BreakVector` (`self.K2_GetActorLocation` _output_get)))
      (set `self.StartingHeight` _returnvalue_z)
      (`self.TrackDamage`))
    (:`Is Not Valid`
      (bind _returnvalue_6 (`GameplayStatics.GetActorOfClass` "/Game/Blueprints/Player/BP_VRPlayer.BP_VRPlayer_C"))
      (`/Engine/EditorBlueprintResources/StandardMacros.IsValid` _returnvalue_6
        (:`Is Valid`
          (set `self.PlayerChar` _returnvalue_6)
          (goto _label))
        (:`Is Not Valid`
          (`KismetSystemLibrary.PrintString` "Found no player class."))))))

(event `TrackDamage`
  (bind _returnvalue (/ (`/Game/FluidFlux/Environment/Readback/BP_FluxDataComponent.FluxFluidHeight` (`self.FluxData`)) 0.485564))
  ;[0.02353 0.02745 0.03529] Update Damage Model
  (bind _returnvalue_2 (`self.ContentDamage` _returnvalue :!label _label_2))
  (set `self.ContentDMG` _returnvalue_2)
  (bind _returnvalue_3 (`self.StructureDamage` _returnvalue))
  (set `self.StructureDMG` _returnvalue_3)
  (`KismetSystemLibrary.Delay` 0.5)
  (goto _label_2))

(event `ToggleSim`
  ;[0.02353 0.02745 0.03529] Play / Pause Simulation
  (`/Game/FluidFlux/Simulation/Blueprints/BP_FluxSimulationDomain.ToggleUpdateSimulation` (`self.SimDomain`))
  (set `self.PlayingSim` (not (`self.PlayingSim`))))

(event `ResetSim`
  ;[0.02353 0.02745 0.03529] Reset Simulation
  (`/Game/FluidFlux/Simulation/Blueprints/BP_FluxSimulationDomain.LoadInitialState` (`self.SimDomain`) "/Game/VFX/Sim2/SimState2.SimState2")
  (for _array_element (`self.Vehicles`)
    (`/Game/VehicleTemplate/Blueprints/SportsCar/AI_Car.ResetCar` _array_element)
    (for _array_element_2 (`self.Humans`)
      (`/Game/Blueprints/NPCs/Humans/AI_Human.ResetHuman` _array_element_2))))

(event `ToggleInundation`
  (params (Showing :type Boolean))
  (bind _buildings (`self.Buildings`))
  (if (`self.ShowingInundation`)
    (for _array_element _buildings
      (bind _returnvalue (`self.GetComponentByClass` _array_element "/Game/Blueprints/AC_DamageCalculator.AC_DamageCalculator_C"))
      (`/Engine/EditorBlueprintResources/StandardMacros.IsValid` _returnvalue
        (:`Is Valid`
          (`/Game/Blueprints/AC_DamageCalculator.DisableInundation` _returnvalue))))
    (else
      (for _array_element_2 _buildings
        (bind _returnvalue_2 (`self.GetComponentByClass` _array_element_2 "/Game/Blueprints/AC_DamageCalculator.AC_DamageCalculator_C"))
        (`/Engine/EditorBlueprintResources/StandardMacros.IsValid` _returnvalue_2
          (:`Is Valid`
            (`/Game/Blueprints/AC_DamageCalculator.ShowInundation` _returnvalue_2))))))
  (set `self.ShowingInundation` (not (`self.ShowingInundation`))))

(event `Timelapse`
  (params (Time :type String))
  (bind _simdomain (`self.SimDomain`))
  (set `/Game/FluidFlux/Simulation/Blueprints/BP_FluxSimulationDomain.IterationsPerSecond` 600 _simdomain)
  (set `/Game/FluidFlux/Simulation/Blueprints/BP_FluxSimulationDomain.IterationsPerFrameMax` 20 _simdomain)
  (`KismetSystemLibrary.Delay` (`KismetStringLibrary.Conv_StringToDouble` Time))
  (set `/Game/FluidFlux/Simulation/Blueprints/BP_FluxSimulationDomain.IterationsPerSecond` 120 _simdomain)
  (set `/Game/FluidFlux/Simulation/Blueprints/BP_FluxSimulationDomain.IterationsPerFrameMax` 4 _simdomain))

(fn `Change Flood Height`
  (params (Delta :type "Float (double-precision)"))
  (`self.K2_AddActorWorldOffset` (`self.Floodmap`) (`KismetMathLibrary.MakeVector` 0.0 0.0 Delta) false false))

(fn `ChangeDischarge`
  (params (Selection :type String))
  (switch `string` Selection
    (:`Low (9600 cfs)`
      (set `self.Discharge` 9600.0))
    (:`Medium (22700 cfs)`
      (set `self.Discharge` 22700.0))
    (:`High (55000 cfs)`
      (set `self.Discharge` 55000.0)))
  (set `/Game/FluidFlux/Simulation/Modifiers/Components/BP_FluxModifierSourceComponent.Volume` (/ (/ (`self.Discharge`) 0.48556) 9600.0) (`self.GetComponentByClass` (`self.SceneMod`) "/Game/FluidFlux/Simulation/Modifiers/Components/BP_FluxModifierSourceComponent.BP_FluxModifierSourceComponent_C")))

(fn `ChangeFog`
  (params (Selection :type String))
  (switch `string` Selection
    (:`None`
      (set `self.FogIntensity` 0.0))
    (:`Light`
      (set `self.FogIntensity` 0.02))
    (:`Heavy`
      (set `self.FogIntensity` 0.1)))
  (`SkyCreator.SetExponentialHeightFogSettings` (`self.SkyRef`) (make `SkyCreatorExponentialHeightFogSettings` (`self.FogIntensity`))))

(fn `ChangeRain`
  (params (Selection :type String))
  (switch `string` Selection
    (:`None`
      (set `self.RainIntensity` 0.0))
    (:`Light`
      (set `self.RainIntensity` 0.5))
    (:`Heavy`
      (set `self.RainIntensity` 1.0)))
  (`SkyCreator.SetWeatherFXSettings` (`self.SkyRef`) (make `SkyCreatorWeatherFXSettings` (`self.RainIntensity`))))

(fn `ChangeTime`
  (params (Selection :type String))
  (switch `string` Selection
    (:`Morning`
      (set `self.SceneTime` 8.0))
    (:`Afternoon`
      (set `self.SceneTime` 12.0))
    (:`Evening`
      (set `self.SceneTime` 20.0)))
  (`SkyCreator.SetTime` (`self.SkyRef`) (`self.SceneTime`)))

(fn `ContentDamage`
  (params (StageHeight :type "Float (double-precision)"))
  (returns (ReturnValue :type "Float (double-precision)"))
  (locals (Intercept :type "Float (double-precision)" :default -134925113.0) (Slope :type "Float (double-precision)" :default 5688154.0))
  (return (`KismetMathLibrary.FMax` 0.0 (+ (* (* StageHeight 0.032808) (`local.Slope`)) (`local.Intercept`)))))

(fn `ResetFloodHeight`
  (bind _floodmap (`self.Floodmap`))
  (bind (_returnvalue_x _returnvalue_y) (`KismetMathLibrary.BreakVector` (`self.K2_GetActorLocation` _floodmap)))
  (`self.K2_SetActorLocation` _floodmap (`KismetMathLibrary.MakeVector` _returnvalue_x _returnvalue_y (`self.StartingHeight`)) false false))

(fn `StructureDamage`
  (params (StageHeight :type "Float (double-precision)"))
  (returns (ReturnValue :type "Float (double-precision)"))
  (locals (Slope :type "Float (double-precision)" :default 3172460.0) (Intercept :type "Float (double-precision)" :default -74897629.0))
  (return (`KismetMathLibrary.FMax` 0.0 (+ (* (* StageHeight 0.032808) (`local.Slope`)) (`local.Intercept`)))))

(fn `TeleportPlayer`
  (params (Index :type Integer))
  (bind _playerchar (`self.PlayerChar`))
  (`self.K2_TeleportTo` _playerchar (`self.K2_GetActorLocation` (`|GetArrayItem` (`self.Waypoints`) Index)) (`self.K2_GetActorRotation` _playerchar)))

(fn `UserConstructionScript`)