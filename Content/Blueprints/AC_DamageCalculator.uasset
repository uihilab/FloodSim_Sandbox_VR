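; Actor component that measures flood inundation on its owning mesh and displays it through a flood damage material.
; It briefly activates the owner's FluxData component, then converts fluid height and bounds-derived mesh height into a clamped 0–1 LocalHeight.
; StartComp polls this in a delay loop until StopComp, which also destroys FluxData on StaticMeshActor owners.
; ShowInundation feeds LocalHeight into a dynamic material; DisableInundation restores the cached original.
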(event `self.ReceiveBeginPlay`
  (bind _returnvalue (`self.GetOwner`))
  ;[0.02353 0.02745 0.03529] Get mesh height and cache references
  (bind _asgm_vrvis (cast `/Game/Blueprints/Core/GM_VRVIS` (`GameplayStatics.GetGameMode`))
    (:`then`
      (set `self.VRGameMode` _asgm_vrvis))
    (:`CastFailed`
      _))
  (set `self.BaseMat` (`PrimitiveComponent.GetMaterial` (`Actor.GetComponentByClass` _returnvalue "/Script/Engine.StaticMeshComponent") 0))
  (set `self.MeshHeight` (* (.z (`.BoxExtent` (`Actor.GetActorBounds` _returnvalue false false))) 2.0))
  (bind _output_get (set `self.FluxData` (`Actor.GetComponentByClass` (`self.GetOwner`) "/Game/FluidFlux/Environment/Readback/BP_FluxDataComponent.BP_FluxDataComponent_C")))
  (`self.Deactivate` _output_get))

(event `GetLocalHeight`
  (bind _fluxdata (`self.FluxData`))
  (`self.Activate` _fluxdata false)
  (`KismetSystemLibrary.Delay` 3.0)
  (set `self.LocalHeight` (`KismetMathLibrary.FClamp` (- 1.0 (/ (/ (* (`/Game/FluidFlux/Environment/Readback/BP_FluxDataComponent.FluxFluidHeight` (`self.FluxData`)) -1.0) (`self.MeshHeight`)) 2.0))))
  (`self.Deactivate` _fluxdata))

(event `StartComp`
  (`/Engine/EditorBlueprintResources/StandardMacros.IsValid` (`self.FluxData`)
    (:`Is Valid`
      _)
    (:`Is Not Valid`
      (set `self.FluxData` (`Actor.GetComponentByClass` (`self.GetOwner`) "/Game/FluidFlux/Environment/Readback/BP_FluxDataComponent.BP_FluxDataComponent_C"))))
  (bind _output_get (set `self.Measuring` true))
  (if _output_get :!label _label
    (`self.GetLocalHeight`)
    (`KismetSystemLibrary.Delay` 1.0)
    (goto _label)
    (else
      (`KismetSystemLibrary.PrintString` "Measurement Stopped"))))

(event `StopComp`
  (set `self.Measuring` false)
  (bind _asstatic_mesh_actor (cast `StaticMeshActor` (`self.GetOwner`)))
  (`self.K2_DestroyComponent` (`Actor.GetComponentByClass` _asstatic_mesh_actor "/Game/FluidFlux/Environment/Readback/BP_FluxDataComponent.BP_FluxDataComponent_C")))

(event `ShowInundation`
  (`self.GetLocalHeight`)
  (`KismetSystemLibrary.Delay` 3.5)
  (bind _returnvalue (`PrimitiveComponent.CreateDynamicMaterialInstance` (`Actor.GetComponentByClass` (`self.GetOwner`) "/Script/Engine.StaticMeshComponent") 0 "/Game/VFX/Mat_FloodDamage.Mat_FloodDamage" "None"))
  (`MaterialInstanceDynamic.SetScalarParameterValue` _returnvalue "LocalHeight" (`self.LocalHeight`)))

(event `DisableInundation`
  (`PrimitiveComponent.SetMaterial` (`Actor.GetComponentByClass` (`self.GetOwner`) "/Script/Engine.StaticMeshComponent") 0 (`self.BaseMat`)))