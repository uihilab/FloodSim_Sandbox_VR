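; BP_FPSPlayer is the desktop first-person player character, flying freely with mouse look, vertical movement and sprint.
; BeginPlay sets Flying movement and adds the IMC_Desktop Enhanced Input context, whose actions drive movement, look and fly speed.
; Main menu, mitigation and analytics inputs share OpenUI, a single-slot toggle that removes any open widget or creates the requested one.
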(event `self.ReceiveBeginPlay`
  (`CharacterMovementComponent.SetMovementMode` (`self.CharacterMovement`) "MOVE_Flying" 0)
  (`EnhancedInputSubsystemInterface.AddMappingContext` (pcsubsystem `EnhancedInputLocalPlayerSubsystem` (`GameplayStatics.GetPlayerController` 0)) "/Game/Blueprints/Player/Input/IMC_Desktop.IMC_Desktop" 0 (struct))
  (`KismetSystemLibrary.PrintString` "Hello"))

(event `EnhancedInput|/Game/Blueprints/Player/Input/IA_MKMove`
  (params (ActionValue :type "Vector2D Structure") (ElapsedSeconds :type "Float (double-precision)") (TriggeredSeconds :type "Float (double-precision)") (InputAction :type "InputAction Object Reference" :default "/Game/Blueprints/Player/Input/IA_MKMove.IA_MKMove"))
  (bind (_x _y) (`KismetMathLibrary.BreakVector2D` ActionValue))
  (:`Triggered`
    (`self.AddMovementInput` (`self.GetActorRightVector`) _x)
    (`self.AddMovementInput` (`self.GetActorForwardVector`) _y)))

(event `EnhancedInput|/Game/Blueprints/Player/Input/IA_VertMove`
  (params (ActionValue :type "Float (double-precision)") (ElapsedSeconds :type "Float (double-precision)") (TriggeredSeconds :type "Float (double-precision)") (InputAction :type "InputAction Object Reference" :default "/Game/Blueprints/Player/Input/IA_VertMove.IA_VertMove"))
  (:`Triggered`
    (`self.AddMovementInput` (`self.GetActorUpVector`) ActionValue)))

(event `EnhancedInput|/Game/Blueprints/Player/Input/IA_OpenControls`
  (params (ActionValue :type Boolean) (ElapsedSeconds :type "Float (double-precision)") (TriggeredSeconds :type "Float (double-precision)") (InputAction :type "InputAction Object Reference" :default "/Game/Blueprints/Player/Input/IA_OpenControls.IA_OpenControls"))
  (:`Started`
    (`self.OpenUI` "/Game/UI/Widgets/UI_MainMenu.UI_MainMenu_C")))

(event `EnhancedInput|/Game/Blueprints/Player/Input/IA_OpenMitigation`
  (params (ActionValue :type Boolean) (ElapsedSeconds :type "Float (double-precision)") (TriggeredSeconds :type "Float (double-precision)") (InputAction :type "InputAction Object Reference" :default "/Game/Blueprints/Player/Input/IA_OpenMitigation.IA_OpenMitigation"))
  (:`Started`
    (`self.OpenUI` "/Game/UI/Widgets/UI_Mitigation.UI_Mitigation_C")))

(event `EnhancedInput|/Game/Blueprints/Player/Input/IA_OpenAnalysis`
  (params (ActionValue :type Boolean) (ElapsedSeconds :type "Float (double-precision)") (TriggeredSeconds :type "Float (double-precision)") (InputAction :type "InputAction Object Reference" :default "/Game/Blueprints/Player/Input/IA_OpenAnalysis.IA_OpenAnalysis"))
  (:`Started`
    (`self.OpenUI` "/Game/UI/Widgets/UI_Analytics.UI_Analytics_C")))

(event `EnhancedInput|/Game/Blueprints/Player/Input/IA_MKSprint`
  (params (ActionValue :type Boolean) (ElapsedSeconds :type "Float (double-precision)") (TriggeredSeconds :type "Float (double-precision)") (InputAction :type "InputAction Object Reference" :default "/Game/Blueprints/Player/Input/IA_MKSprint.IA_MKSprint"))
  (bind _charactermovement (`self.CharacterMovement`))
  (:`Started`
    (set `CharacterMovementComponent.MaxFlySpeed` 2400.0 _charactermovement))
  (:`Completed`
    (set `CharacterMovementComponent.MaxFlySpeed` 1200.0 _charactermovement)))

(event `EnhancedInput|/Game/Blueprints/Player/Input/IA_MKLook`
  (params (ActionValue :type "Vector2D Structure") (ElapsedSeconds :type "Float (double-precision)") (TriggeredSeconds :type "Float (double-precision)") (InputAction :type "InputAction Object Reference" :default "/Game/Blueprints/Player/Input/IA_MKLook.IA_MKLook"))
  (:`Triggered`
    (`self.AddControllerYawInput` ActionValue_X)
    (`self.AddControllerPitchInput` (* ActionValue_Y -1.0))))

(fn `OpenUI`
  (params (Widget :type "UserWidget Class Reference"))
  (if (`self.UIOpen`)
    (`Widget.RemoveFromParent` (`self.UI_Ref`))
    (set `self.UIOpen` false)
    (else
      (bind _returnvalue (`|CreateWidget` Widget))
      (bind _output_get (set `self.UI_Ref` _returnvalue))
      (`UserWidget.AddToViewport` _returnvalue 0)
      (`UserWidget.AddToViewport` _output_get 0)
      (set `self.UIOpen` true))))

(fn `UserConstructionScript`)